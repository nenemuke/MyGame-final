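; BP_CheckPoint is a checkpoint that updates the player's respawn location the first time player 0 overlaps its Box.
; It passes the location to BP_UnrealQuest3_Mode via SetNewSpawnLocation, sets AlreadyPassed and prints a message.
; CheckRespawnLocation line-traces down for the ground and adds the player's capsule half-height.
; On a miss, it adds a fixed height to the trace's hit location rather than the actor's position.
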(event `self.Box.OnComponentBeginOverlap`
  (params (OverlappedComponent :type "PrimitiveComponent Object Reference") (OtherActor :type "Actor Object Reference") (OtherComp :type "PrimitiveComponent Object Reference") (OtherBodyIndex :type Integer) (bFromSweep :type Boolean) (SweepResult :type "HitResult Structure (by ref)"))
  (if (and (== OtherActor (`GameplayStatics.GetPlayerCharacter` 0)) (not (`self.AlreadyPassed`)))
    ;[1 1 1] チェックポイントを踏むとGameModeにリスポーン位置を渡す
    (bind _asbp_unreal_quest_3_mode (cast `/Game/Unreal/UnrealQuest3/Blueprints/BP_UnrealQuest3_Mode` (`GameplayStatics.GetGameMode`)))
    (bind _location (`self.CheckRespawnLocation` :!pinned true)) ; チェックポイントの地面の高さをチェック
    (`/Game/Unreal/UnrealQuest3/Blueprints/BP_UnrealQuest3_Mode.SetNewSpawnLocation` _asbp_unreal_quest_3_mode _location)
    (set `self.AlreadyPassed` true)
    (`KismetSystemLibrary.PrintString` "CheckPoint通過！")))

(fn `CheckRespawnLocation`
  (returns (Location :type "Vector Structure"))
  (bind _returnvalue (`self.K2_GetActorLocation`))
  (bind _returnvalue_2 (`self.GetActorUpVector`))
  (bind (_outhit _returnvalue_3) (`KismetSystemLibrary.LineTraceSingle` (+ _returnvalue (* _returnvalue_2 100.0)) (+ _returnvalue (* _returnvalue_2 -1000.0)) "TraceTypeQuery1"))
  (if _returnvalue_3
    (bind (_bblockinghit _binitialoverlap _time _distance _location) (`GameplayStatics.BreakHitResult` _outhit))
    (return (+ _location (`KismetMathLibrary.MakeVector` 0.0 0.0 (`CapsuleComponent.CapsuleHalfHeight` (`Character.CapsuleComponent` (`GameplayStatics.GetPlayerCharacter` 0))))))
    (else
      (return (+ _location (0.0 0.0 200.0))))))

(fn `UserConstructionScript`)