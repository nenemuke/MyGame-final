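; BP_Goal is a stage goal trigger that moves the game to another level when the player enters it.
; When the player character overlaps its Box, it checks TargetLevel and, only once, calls ChangeStage on BP_UnrealQuest3_Mode with that level and GoalBGM.
; The level switch is delegated to the GameMode so it can run its own processing.
; An unset TargetLevel prints a warning naming the actor instead.
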(event `self.Box.OnComponentBeginOverlap`
  (params (OverlappedComponent :type "PrimitiveComponent Object Reference") (OtherActor :type "Actor Object Reference") (OtherComp :type "PrimitiveComponent Object Reference") (OtherBodyIndex :type Integer) (bFromSweep :type Boolean) (SweepResult :type "HitResult Structure (by ref)"))
  (if (== OtherActor (`GameplayStatics.GetPlayerCharacter` 0))
    (`self.TargetLevel` :!pinned true ; 変数にLevelが設定されているかどうかチェック
      (:`then`
        (`/Engine/EditorBlueprintResources/StandardMacros.DoOnce` false
          (:`Completed`
            ;[0 0 0] GameModeのレベル切り替え処理を呼び出し。(GameMode側で行いたい処理があるため)
            (bind _asbp_unreal_quest_3_mode (cast `/Game/Unreal/UnrealQuest3/Blueprints/BP_UnrealQuest3_Mode` (`GameplayStatics.GetGameMode`)))
            (`/Game/Unreal/UnrealQuest3/Blueprints/BP_UnrealQuest3_Mode.ChangeStage` _asbp_unreal_quest_3_mode (`self.GoalBGM`) (`self.TargetLevel`)))))
      (:`else`
        (`KismetSystemLibrary.PrintString` (`KismetStringLibrary.Concat_StrStr` (`KismetSystemLibrary.GetDisplayName` self) "のTargetLevelにLevelが設定されていません。") true true (struct :`R` 1.0 :`B` 0.182568 :`A` 1.0) :!pinned true) ; 変数にLevelが設定されていなければPrintStringで警告
      ))))

(fn `UserConstructionScript`)