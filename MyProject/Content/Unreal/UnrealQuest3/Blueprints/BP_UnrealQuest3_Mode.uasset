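; Game mode for UnrealQuest3 that handles player respawning, stage changes and background music.
; It binds to the player character's OnDestroyed, restarts at the stored checkpoint or at the PlayerStart if none is set, then rebinds for the next death.
; ChangeStage fades in new music if the track differs, disables input, unbinds the death event, then after a timer opens the level and clears the checkpoint.
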(event `self.ReceiveBeginPlay`
  (add `self.OnDestroyed` (`GameplayStatics.GetPlayerCharacter` 0) (delegate `DestroyedPlayer`) :!pinned true :!label _label) ; プレイヤー死亡時にイベントを発行
  ;[1 1 1] ゲーム開始時のBGM再生
  (`AudioComponent.Play` (`self.Audio`) 0.0))

(event `Respawned`
  (goto _label))

(event `DestroyedPlayer` :!signature `self.OnDestroyed`
  (params (DestroyedActor :type "Actor Object Reference"))
  ;[1 1 1] Playerの死亡時にリスポーン処理を実行
  (if (not (== (`self.SpawnTransform`) (0.0 0.0 0.0))) :!pinned true
    (`self.RestartPlayerAtTransform` (`GameplayStatics.GetPlayerController` 0) (`KismetMathLibrary.MakeTransform` (`self.SpawnTransform`) (struct :`Yaw` -90.0)) :!pinned true) ; チェックポイントによるスポーン位置に変更があればそちらにリスポーン
    (else
      (`self.RestartPlayer` (`GameplayStatics.GetPlayerController` 0) :!pinned true) ; 初期位置ならプレイヤースタートからリスポーン
    ))
  (`self.Respawned` :!pinned true) ; リスポーン後にプレイヤーの死亡通知を際バインド
)

(event `SetNewSpawnLocation`
  (params (NewSpawnTransform :type "Vector Structure"))
  ;[1 1 1] Spawn位置を更新
  (set `self.SpawnTransform` NewSpawnTransform))

(event `ChangeStage`
  (params (SoundCue :type "SoundCue Object Reference") (Level :type "World Soft Object Reference"))
  ;[1 1 1] レベルの変更処理。変更時にSpawn位置を初期化
  ; BGMの鳴らし分けの処理
  (`|ExecutionSequence`
    (:`then_0`
      (if (!= (`self.CurrentBGM_ObjectName`) SoundCue) :!pinned true
        (`AudioComponent.Stop` (`self.Audio`))
        (bind _output_get (set `self.CurrentBGM_ObjectName` SoundCue))
        (`AudioComponent.SetSound` (`self.Audio`) _output_get)
        (`AudioComponent.FadeIn` (`self.Audio`) 1.0 1.0 0.0 "Linear")))
    (:`then_1`
      (`self.DisableInput` (`GameplayStatics.GetPlayerCharacter` 0) (`GameplayStatics.GetPlayerController` 0))
      (`KismetSystemLibrary.K2_SetTimerDelegate` (delegate `ChangeLevel`) 3.0)
      ;;[0 0 0] 現在のリスタート処理用のバインドを解除しておく
      (clear `self.OnDestroyed` (`GameplayStatics.GetPlayerCharacter` 0)))))

(event `ChangeLevel`
  ;[1 1 1] レベルの変更処理。変更時にSpawn位置を初期化
  ; BGMの鳴らし分けの処理
  ;;[0 0 0] レベルの切り替え
  (`GameplayStatics.OpenLevelBySoftObjectPtr` (stale `ChangeStage` Level))
  (set `self.SpawnTransform` (0.0 0.0 0.0) :!pinned true) ; スポーン位置の初期化
)

(fn `UserConstructionScript`)