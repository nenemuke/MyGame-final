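; BP_Ring is a ring gimmick that shows a Niagara fire effect while the player character is inside its trigger box.
; Begin overlap activates Niagara and restarts the FireControl timeline, which feeds its inverted rate into User.MaskAmount so flames rise from bottom to top.
; End overlap deactivates the effect.
; The construction script passes the static mesh's local bounds to Niagara for the effect.
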(event `self.Box.OnComponentBeginOverlap`
  (params (OverlappedComponent :type "PrimitiveComponent Object Reference") (OtherActor :type "Actor Object Reference") (OtherComp :type "PrimitiveComponent Object Reference") (OtherBodyIndex :type Integer) (bFromSweep :type Boolean) (SweepResult :type "HitResult Structure (by ref)"))
  (if (== OtherActor (`GameplayStatics.GetPlayerCharacter` 0))
    ;[1 1 1] Triggerに入ったか出たかでNiagaraをオンオフ
    (`ActorComponent.SetActive` (`self.Niagara`) true false)
    ;[1 1 1] 炎を下から上へ発生させるためにNiagaraのMask処理用パラメーターを渡す処理
    (bind (_direction _rate) (`Timeline|FireControl` :!via `PlayFromStart`)
      (:`Update`
        (`NiagaraComponent.SetVariableFloat` (`self.Niagara`) "User.MaskAmount" (`KismetMathLibrary.Abs` (- 1.0 _rate)))))))

(event `self.Box.OnComponentEndOverlap`
  (params (OverlappedComponent :type "PrimitiveComponent Object Reference") (OtherActor :type "Actor Object Reference") (OtherComp :type "PrimitiveComponent Object Reference") (OtherBodyIndex :type Integer))
  (if (== OtherActor (`GameplayStatics.GetPlayerCharacter` 0))
    ;[1 1 1] Triggerに入ったか出たかでNiagaraをオンオフ
    (`ActorComponent.SetActive` (`self.Niagara`) false false)))

(fn `UserConstructionScript`
  (bind _niagara (`self.Niagara`))
  (bind (_min _max) (`StaticMeshComponent.GetLocalBounds` (`self.StaticMesh`)))
  ;[1 1 1] NiagaraにMeshのBoundsを渡す
  (`NiagaraComponent.SetVariableVec3` _niagara "User.ObjectBoundsMin" _min)
  (`NiagaraComponent.SetVariableVec3` _niagara "User.ObjectBoundsMax" _max))