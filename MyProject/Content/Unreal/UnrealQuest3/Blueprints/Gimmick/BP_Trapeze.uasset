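; BP_Trapeze is a gimmick that moves a static mesh back and forth along a spline while the player is inside its trigger box.
; Overlap starts the MoveControl timeline, whose Rate drives the mesh's distance along the spline.
; Each finish flips IsBackward, which mirrors Rate for the return leg, and replays if the player remains inside.
; The construction script divides the timeline play rate by MoveSpeed, making it a travel duration.
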(event `self.Box.OnComponentBeginOverlap`
  (params (OverlappedComponent :type "PrimitiveComponent Object Reference") (OtherActor :type "Actor Object Reference") (OtherComp :type "PrimitiveComponent Object Reference") (OtherBodyIndex :type Integer) (bFromSweep :type Boolean) (SweepResult :type "HitResult Structure (by ref)"))
  ;[1 1 1] 動きを開始する処理とPlayerがTrigger内にいるかどうかで継続して動かすかを決める処理
  (if (== OtherActor (`GameplayStatics.GetPlayerCharacter` 0))
    (if (not (`TimelineComponent.IsPlaying` (`self.MoveControl`))) :!pinned true
      (`TimelineComponent.PlayFromStart` (`self.MoveControl`))
      ;;[0 0 0] シーソーのループ再生フラグの変更
      (set `self.PlayerIsInArea` true))))

(event `self.Box.OnComponentEndOverlap`
  (params (OverlappedComponent :type "PrimitiveComponent Object Reference") (OtherActor :type "Actor Object Reference") (OtherComp :type "PrimitiveComponent Object Reference") (OtherBodyIndex :type Integer))
  ;[1 1 1] 動きを開始する処理とPlayerがTrigger内にいるかどうかで継続して動かすかを決める処理
  (if (== OtherActor (`GameplayStatics.GetPlayerCharacter` 0))
    ;;[0 0 0] シーソーのループ再生フラグの変更
    (set `self.PlayerIsInArea` false)))

(fn `UserConstructionScript`
  ;[0 0 0] 秒数で往復にかかる時間を指定
  (`TimelineComponent.SetPlayRate` (`self.MoveControl`) (/ (`TimelineComponent.GetPlayRate` (`self.MoveControl`)) (`self.MoveSpeed`))))