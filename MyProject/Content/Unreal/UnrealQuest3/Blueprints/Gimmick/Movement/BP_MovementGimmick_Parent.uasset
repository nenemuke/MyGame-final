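; BP_MovementGimmick_Parent is a parent Blueprint for moving gimmicks that travel between two points via an InterpToMovement component.
; Its Construction Script rebuilds the control points from StartLocation and EndLocation as relative positions, then applies MoveDuration as the component's duration.
; IsMove sets whether the movement auto-activates.
; These settings are exposed as variables so placed gimmicks are easy to configure and preview.
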(fn `UserConstructionScript`
  (`|ExecutionSequence`
    (:`then_0`
      ;[1 1 1] 設定をプレビューしやすいようにLocationの設定などを外部へ公開
      (`KismetArrayLibrary.Array_Clear` (`InterpToMovementComponent.ControlPoints` (`self.InterpToMovement`)))
      (`InterpToMovementComponent.AddControlPointPosition` (`self.InterpToMovement`) (`self.StartLocation`) true)
      (`InterpToMovementComponent.AddControlPointPosition` (`self.InterpToMovement`) (`self.EndLocation`) true))
    (:`then_1`
      (set `InterpToMovementComponent.Duration` (`self.Move Duration`) (`self.InterpToMovement`)))
    (:`then_2`
      (`ActorComponent.SetAutoActivate` (`self.InterpToMovement`) (`self.IsMove`)))))